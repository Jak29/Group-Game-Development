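; BP_Enemy is an AI-controlled enemy that spots the player, attacks, and can drop bandages on death.
; Pawn sensing sets the hasSeenPlayer blackboard flag when it sees BP_Player, handing that knowledge to the AI controller's blackboard.
; The Attack event waits a delay, then spawns a BP_EnemyAttack at the enemy's location and rotation.
; Damage reduces Health; at zero the actor is destroyed, with a random chance to spawn BP_Bandage.
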(event OnSeePawn(PawnSensing)
  (params (Pawn :type Pawn%20Object%20Reference))
  (Utilities|Casting|CastToBP_Player Pawn)
  (AI|Components|Blackboard|SetValueasBool (AI|GetBlackboard (AI|GetAIController self)) (Utilities|Name|MakeLiteralName "hasSeenPlayer") true))

(event Custom|Attack
  (Utilities|FlowControl|Delay (Variables|Default|GetattackDelay))
  (Game|SpawnActorfromClass "/Game/GroupProject/AI/BP_EnemyAttack.BP_EnemyAttack_C" (Math|Transform|MakeTransform (Transformation|GetActorLocation) (Transformation|GetActorRotation) "1.000000,1.000000,1.000000") "Undefined" "MultiplyWithRoot" 0 0))

(event EventBeginPlay)

(event Collision|EventActorBeginOverlap
  (params (OtherActor :type Actor%20Object%20Reference)))

(event EventTick
  (params (DeltaSeconds :type Float%20%28single-precision%29)))

(event Game|Damage|EventAnyDamage
  (params (Damage :type Float%20%28single-precision%29) (DamageType :type Damage%20Type%20Object%20Reference) (InstigatedBy :type Controller%20Object%20Reference) (DamageCauser :type Actor%20Object%20Reference))
  (Variables|Default|Sethealth (- (Variables|Default|Gethealth) Damage))
  (if (<= (Variables|Default|Gethealth) 0.0)
    (Actor|DestroyActor)
    (if (<= (Math|Random|RandomFloatinRange 0.0 1.0) (Variables|Default|GetbandageDropChance))
      (Game|SpawnActorfromClass "/Game/GroupProject/Items/BP_Bandage.BP_Bandage_C" (Math|Transform|MakeTransform (Transformation|GetActorLocation) "0, 0, 0" "1.000000,1.000000,1.000000") "Undefined" "MultiplyWithRoot" 0 0))))

(fn ConstructionScript)