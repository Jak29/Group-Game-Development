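; BP_ForwardGate is a level transition gate that sends the player to Level_1 when its trigger is overlapped.
; On overlap it copies the player's Health and Stamina into BP_GameInstance so they persist across the level load.
; It then shows a W_LevelFade widget with a fade-in animation and opens the level after a short delay.
; The overlap event does not filter which actor entered the trigger.
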(event OnComponentBeginOverlap(Trigger)
  (params (OverlappedComponent :type Primitive%20Component%20Object%20Reference) (OtherActor :type Actor%20Object%20Reference) (OtherComp :type Primitive%20Component%20Object%20Reference) (OtherBodyIndex :type Integer) (bFromSweep :type Boolean) (SweepResult :type Hit%20Result%20Structure%20%28by%20ref%29))
  (CallFunction|SaveData)
  (bind _returnvalue (UserInterface|CreateWidget "/Game/GroupProject/UserInterface/W_LevelFade.W_LevelFade_C"))
  (UserInterface|Viewport|AddtoViewport _returnvalue 0)
  (Default|FadeinAnimation _returnvalue)
  (Utilities|FlowControl|Delay 0.5)
  (Game|OpenLevel(byObjectReference) "/Game/GroupProject/Levels/Level_1.Level_1"))

(event EventBeginPlay)

(event Collision|EventActorBeginOverlap
  (params (OtherActor :type Actor%20Object%20Reference)))

(event EventTick
  (params (DeltaSeconds :type Float%20%28single-precision%29)))

(fn ConstructionScript)

(fn SaveData
  (bind _asbp_player (Utilities|Casting|CastToBP_Player (Game|GetPlayerCharacter 0)))
  (bind _asbp_game_instance (Utilities|Casting|CastToBP_GameInstance (Game|GetGameInstance)))
  (Variables|/Game/GroupProject/GameModes/BP_GameInstance.BP_GameInstance_C|Setstamina _asbp_game_instance (Variables|/Game/GroupProject/Player/BP_Player.BP_Player_C|Getstamina _asbp_player))
  (Variables|/Game/GroupProject/GameModes/BP_GameInstance.BP_GameInstance_C|Sethealth _asbp_game_instance (Variables|/Game/GroupProject/Player/BP_Player.BP_Player_C|Gethealth _asbp_player)))